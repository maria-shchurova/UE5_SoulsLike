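; Gameplay ability that puts the owning BP_CrossroadsCharacter into a blocking state.
; On activation it commits, applies GE_IsBlocking to the owner and calls the character's Blocking function.
; A WaitGameplayTagRemove task on Character.IsBlocking ends the ability when that tag is removed.
; On end it calls FinishedBlocking on the character and shuts down the stored wait task.
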(event `self.K2_ActivateAbility`
  (`self.K2_CommitAbility`)
  (`self.BP_ApplyGameplayEffectToOwner` "/Game/ProjectFolder/Blueprints/Abilities/GE_IsBlocking.GE_IsBlocking_C")
  (bind _asbp_crossroads_character (cast `/Game/ThirdPerson/Blueprints/BP_CrossroadsCharacter` (`.OwnerActor` (break `GameplayAbilityActorInfo` (`self.GetActorInfo`)))))
  (`/Game/ThirdPerson/Blueprints/BP_CrossroadsCharacter.Blocking` _asbp_crossroads_character)
  (bind _asynctaskproxy (`AbilityTask_WaitGameplayTagRemoved.WaitGameplayTagRemove` (struct :`TagName` "Character.IsBlocking") null)
    (:`then`
      (set `self.Async Wait For Tag Removal` _asynctaskproxy))
    (:`Removed`
      (`self.K2_EndAbility`))))

(event `self.K2_OnEndAbility`
  (params (bWasCancelled :type Boolean))
  (bind _async_wait_for_tag_removal (`self.Async Wait For Tag Removal`))
  (`/Game/ThirdPerson/Blueprints/BP_CrossroadsCharacter.FinishedBlocking` (stale `self.K2_ActivateAbility` _asbp_crossroads_character))
  (`/Engine/EditorBlueprintResources/StandardMacros.IsValid` _async_wait_for_tag_removal
    (:`Is Valid`
      (`GameplayTask.EndTask` _async_wait_for_tag_removal))))